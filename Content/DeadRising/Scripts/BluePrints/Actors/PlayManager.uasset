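; PlayManager is an actor that handles screen transitions into and out of a gameplay level.
; On BeginPlay it creates TransWidget, adds it to the viewport and plays the opening transition.
; Timelines animate the Offset parameter on the widget's retainer box effect material, forward to open and in reverse to close.
; TransClose and TransCloseTitle load ResultMap and TitleMap respectively when their reversed timelines finish.
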(event `self.ReceiveBeginPlay`
  (`|ExecutionSequence`
    (:`then_0`
      (bind _returnvalue (`|CreateWidget` "/Game/DeadRising/Scripts/BluePrints/UIs/Widget/TransWidget.TransWidget_C"))
      (bind _output_get (set `self.TransWidget` _returnvalue))
      (`UserWidget.AddToViewport` _output_get 0))
    (:`then_1`
      (`self.TransOpen`))))

(event `TransClose`
  ;[0.8073 0.6003 0.3455] TransClose
  (`|ExecutionSequence`
    (:`then_0`
      (bind (_direction _offset) (`Timeline|TL_Close` :!via `ReverseFromEnd`)
        (:`Update`
          (`MaterialInstanceDynamic.SetScalarParameterValue` (`RetainerBox.GetEffectMaterial` (`/Game/DeadRising/Scripts/BluePrints/UIs/Widget/TransWidget.RetainerBox_TransImage` (`self.TransWidget`))) "Offset" _offset))
        (:`Finished`
          (`GameplayStatics.OpenLevel` "ResultMap"))))))

(event `TransOpen`
  ;[0.4158 0.6112 1] TransOpen
  (`|ExecutionSequence`
    (:`then_0`
      (bind (_direction _offset) (`Timeline|TL_Open` :!via `PlayFromStart`)
        (:`Update`
          (`MaterialInstanceDynamic.SetScalarParameterValue` (`RetainerBox.GetEffectMaterial` (`/Game/DeadRising/Scripts/BluePrints/UIs/Widget/TransWidget.RetainerBox_TransImage` (`self.TransWidget`))) "Offset" _offset))))))

(event `TransCloseTitle`
  (`|ExecutionSequence`
    (:`then_0`
      (bind (_direction _offset) (`Timeline|TL_TransClose` :!via `ReverseFromEnd`)
        (:`Update`
          (`MaterialInstanceDynamic.SetScalarParameterValue` (`RetainerBox.GetEffectMaterial` (`/Game/DeadRising/Scripts/BluePrints/UIs/Widget/TransWidget.RetainerBox_TransImage` (`self.TransWidget`))) "Offset" _offset))
        (:`Finished`
          (`GameplayStatics.OpenLevel` "TitleMap"))))))

(fn `UserConstructionScript`)