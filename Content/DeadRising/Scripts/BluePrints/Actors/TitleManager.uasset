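; TitleManager is an actor that runs screen transitions for the title, including the handoff into PlayMap.
; TransOpen and TransClose each create a TransWidget, then use a timeline to drive the Offset parameter on its RetainerBox effect material.
; TransClose plays its timeline in reverse from the end and opens PlayMap when finished.
; BeginPlay and Tick are empty, and the only internal calls to both transitions sit in disconnected graphs.
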(event `Key|LeftMouseButton`
  (params (Key :type "Key Structure")))

(event `self.ReceiveTick`
  (params (DeltaSeconds :type "Float (single-precision)")))

(event `self.ReceiveBeginPlay`)

(event `TransClose`
  ;[0.8073 0.6003 0.3455] TransClose
  (bind _returnvalue (`|CreateWidget` "/Game/DeadRising/Scripts/BluePrints/UIs/Widget/TransWidget.TransWidget_C"))
  (bind _output_get (set `self.TransWidget` _returnvalue))
  (`UserWidget.AddToViewport` _output_get 0)
  (`|ExecutionSequence`
    (:`then_0`
      (bind (_direction _offset) (`Timeline|TL_Close` :!via `ReverseFromEnd`)
        (:`Update`
          (`MaterialInstanceDynamic.SetScalarParameterValue` (`RetainerBox.GetEffectMaterial` (`/Game/DeadRising/Scripts/BluePrints/UIs/Widget/TransWidget.RetainerBox_TransImage` _output_get)) "Offset" _offset))
        (:`Finished`
          (`GameplayStatics.OpenLevel` "PlayMap"))))))

(event `TransOpen`
  ;[0.4158 0.6112 1] TransOpen
  (bind _returnvalue (`|CreateWidget` "/Game/DeadRising/Scripts/BluePrints/UIs/Widget/TransWidget.TransWidget_C"))
  (bind _output_get (set `self.TransWidget` _returnvalue))
  (`UserWidget.AddToViewport` _output_get 0)
  (`|ExecutionSequence`
    (:`then_0`
      (bind (_direction _offset) (`Timeline|TL_Open` :!via `PlayFromStart`)
        (:`Update`
          (`MaterialInstanceDynamic.SetScalarParameterValue` (`RetainerBox.GetEffectMaterial` (`/Game/DeadRising/Scripts/BluePrints/UIs/Widget/TransWidget.RetainerBox_TransImage` _output_get)) "Offset" _offset))))))

(fn `UserConstructionScript`)