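; Camera actor for the game over screen, judging by its name, that slowly pans its spring arm in one direction.
; Each tick, MoveCamera adds a fixed rotation step to the arm's world yaw and clamps it to a configured range, keeping pitch and roll.
; The step is not scaled by delta time, so pan speed depends on frame rate.
; BeginPlay enables player input, though no input events are handled.
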(event `self.ReceiveBeginPlay`
  (`self.EnableInput` (`GameplayStatics.GetPlayerController` 0)))

(event `self.ReceiveTick`
  (params (DeltaSeconds :type "Float (single-precision)"))
  (`self.MoveCamera` 1.0))

(fn `MoveCamera`
  (params (MovingDirection :type "Float (double-precision)"))
  (bind (_returnvalue_roll _returnvalue_pitch _returnvalue_yaw) (`KismetMathLibrary.BreakRotator` (`SceneComponent.K2_GetComponentRotation` (`self.SpringArm`))))
  (bind (_returnvalue_roll_2 _returnvalue_pitch_2) (`KismetMathLibrary.BreakRotator` (`SceneComponent.K2_GetComponentRotation` (`self.SpringArm`))))
  (`SceneComponent.K2_SetWorldRotation` (`self.SpringArm`) (`KismetMathLibrary.MakeRotator` _returnvalue_roll_2 _returnvalue_pitch_2 (`KismetMathLibrary.FClamp` (+ (* MovingDirection (`self.CameraRotationSpeed`)) _returnvalue_yaw) (`self.RotationRangeMin`) (`self.RotationRangeMax`))) false false))

(fn `UserConstructionScript`)