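; ResultManager is an actor that runs screen transitions for entering and leaving a level, presumably the result screen.
; On BeginPlay it creates TransWidget, adds it to the viewport and plays TransOpen, hiding the widget when finished.
; TransClose shows the widget, plays its own timeline in reverse, then opens the named level.
; Both timelines animate the Offset parameter on the widget's retainer box effect material.
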(event `self.ReceiveBeginPlay`
  (`|ExecutionSequence`
    (:`then_0`
      (bind _returnvalue (`|CreateWidget` "/Game/DeadRising/Scripts/BluePrints/UIs/Widget/TransWidget.TransWidget_C"))
      (bind _output_get (set `self.TransWidget` _returnvalue))
      (`UserWidget.AddToViewport` _output_get 1))
    (:`then_1`
      (`self.TransOpen`))))

(event `TransClose`
  (params (LevelName :type Name))
  ;[0.8073 0.6003 0.3455] TransClose
  (`Widget.SetVisibility` (`self.TransWidget`) "Visible")
  (bind (_direction _offset) (`Timeline|TL_TransClose` :!via `ReverseFromEnd`)
    (:`Update`
      (`MaterialInstanceDynamic.SetScalarParameterValue` (`RetainerBox.GetEffectMaterial` (`/Game/DeadRising/Scripts/BluePrints/UIs/Widget/TransWidget.RetainerBox_TransImage` (`self.TransWidget`))) "Offset" _offset))
    (:`Finished`
      (`GameplayStatics.OpenLevel` LevelName))))

(event `TransOpen`
  (bind _transwidget (`self.TransWidget`))
  ;[0.4158 0.6112 1] TransOpen
  (bind (_direction _offset) (`Timeline|TL_TransOpen` :!via `PlayFromStart`)
    (:`Update`
      (`MaterialInstanceDynamic.SetScalarParameterValue` (`RetainerBox.GetEffectMaterial` (`/Game/DeadRising/Scripts/BluePrints/UIs/Widget/TransWidget.RetainerBox_TransImage` _transwidget)) "Offset" _offset))
    (:`Finished`
      (`Widget.SetVisibility` _transwidget "Hidden"))))

(fn `UserConstructionScript`)