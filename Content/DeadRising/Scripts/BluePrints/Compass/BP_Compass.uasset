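; BP_Compass puts the compass HUD on screen and manages a toggleable location marker for it.
; On BeginPlay it creates the UI_Compass widget and adds it to the viewport.
; The compassMarker event uses a FlipFlop to alternate between spawning a BP_LocationMarker at the player pawn's location, passing that point to the widget, and disabling the widget's marker while destroying the actor.
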(event `self.ReceiveBeginPlay`
  (bind _returnvalue (`|CreateWidget` "/Game/DeadRising/Scripts/BluePrints/Compass/UI_Compass.UI_Compass_C"))
  (bind _output_get (set `self.CompassWidget` _returnvalue))
  (`UserWidget.AddToViewport` _output_get 0))

(event `self.ReceiveTick`
  (params (DeltaSeconds :type "Float (single-precision)")))

(event `compassMarker`
  (`/Engine/EditorBlueprintResources/StandardMacros.FlipFlop`
    (:`A`
      (bind _returnvalue (`|SpawnActorFromClass` "/Game/DeadRising/Scripts/BluePrints/Compass/BP_LocationMarker.BP_LocationMarker_C" (`KismetMathLibrary.MakeTransform` (`Actor.K2_GetActorLocation` (`GameplayStatics.GetPlayerPawn` 0))) "Undefined" "OverrideRootScale" null null))
      (bind _output_get (set `self.LocationMarker` _returnvalue))
      (`/Game/DeadRising/Scripts/BluePrints/Compass/UI_Compass.SetLocationMarker` (`self.CompassWidget`) (`Actor.K2_GetActorLocation` _output_get) true))
    (:`B`
      (`/Game/DeadRising/Scripts/BluePrints/Compass/UI_Compass.SetLocationMarker` (`self.CompassWidget`) (0.0 0.0 0.0) false)
      (`Actor.K2_DestroyActor` (`self.LocationMarker`)))))