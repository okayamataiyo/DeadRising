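; BP_Propeller is a helicopter rotor actor that spins up and then lifts off.
; Once the externally set IsTorigger flag is true, a DoOnce starts rotation and engine-start audio, then uses delays to play flight audio and enable flying.
; Tick adds capped, gradually increasing increments to yaw and, when flying, to Z, without delta-time scaling, so motion is frame-rate dependent.
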(event `self.ReceiveTick`
  (params (DeltaSeconds :type "Float (single-precision)"))
  (bind (_returnvalue_x _returnvalue_y _returnvalue_z) (`KismetMathLibrary.BreakVector` (`self.K2_GetActorLocation`)))
  (bind (_returnvalue_roll _returnvalue_pitch _returnvalue_yaw) (`KismetMathLibrary.BreakRotator` (`self.K2_GetActorRotation`)))
  (bind _rotvalue (`self.RotValue`))
  (bind _flyvalue (`self.FlyValue`))
  (`|ExecutionSequence`
    (:`then_0`
      (if (`self.IsRotStart`)
        (if (<= _rotvalue 1000.0)
          (set `self.RotValue` (+ _rotvalue 0.1)))
        (`self.K2_SetActorRotation` (`KismetMathLibrary.MakeRotator` _returnvalue_roll _returnvalue_pitch (+ _returnvalue_yaw (`self.RotValue`))))
        (if (stale _output_get)
          (if (<= _flyvalue 20.0)
            (set `self.FlyValue` (+ _flyvalue 0.01)))
          (`self.K2_SetActorLocation` (`KismetMathLibrary.MakeVector` _returnvalue_x _returnvalue_y (+ _returnvalue_z (`self.FlyValue`)))))))
    (:`then_1`
      (if (`self.IsTorigger`)
        (`/Engine/EditorBlueprintResources/StandardMacros.DoOnce` false
          (:`Completed`
            (set `self.IsRotStart` true)
            (`GameplayStatics.PlaySound2D` "/Game/DeadRising/Resources/Music/ヘリコプターエンジン始動（機外）__2_.ヘリコプターエンジン始動（機外）__2_" 1.0 1.0 0.0 null null)
            (`KismetSystemLibrary.Delay` 4.0)
            (`GameplayStatics.PlaySound2D` "/Game/DeadRising/Resources/Music/ヘリコプター飛行中（機外）.ヘリコプター飛行中（機外）" 1.0 1.0 0.0 null null)
            (`KismetSystemLibrary.Delay` 4.0)
            (bind _output_get (set `self.IsFlying` true))))))))

(fn `UserConstructionScript`)