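; BP_Propeller_2 is a propeller actor that spins up once the BP_Propeller actor starts rotating.
; Every Tick it finds that actor with GetActorOfClass and latches its own IsRotStart on when the other's is set, with no path to clear it.
; While latched, it grows RotValue up to a cap and adds it to actor pitch each frame, so the spin accelerates without delta-time scaling.
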(event `self.ReceiveTick`
  (params (DeltaSeconds :type "Float (single-precision)"))
  (bind (_returnvalue_roll _returnvalue_pitch _returnvalue_yaw) (`KismetMathLibrary.BreakRotator` (`self.K2_GetActorRotation`)))
  (bind _rotvalue (`self.RotValue`))
  (`|ExecutionSequence`
    (:`then_0`
      (if (`self.IsRotStart`)
        (if (<= _rotvalue 1000.0)
          (set `self.RotValue` (+ _rotvalue 0.1)))
        (`self.K2_SetActorRotation` (`KismetMathLibrary.MakeRotator` _returnvalue_roll (+ _returnvalue_pitch (`self.RotValue`)) _returnvalue_yaw))))
    (:`then_1`
      (bind _returnvalue (`GameplayStatics.GetActorOfClass` "/Game/DeadRising/BP_Propeller.BP_Propeller_C"))
      (if (`/Game/DeadRising/BP_Propeller.IsRotStart` _returnvalue)
        (set `self.IsRotStart` true)))))

(fn `UserConstructionScript`)